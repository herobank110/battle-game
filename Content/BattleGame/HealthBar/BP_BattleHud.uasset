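; BP_BattleHud is the battle HUD that puts the main UMG widget on screen and shows the player character's health.
; On BeginPlay it creates WBP_BattleHud for the owning player, adds it to the viewport and caches the controlled pawn as a BattleGameCharacter.
; Each Tick it polls that character's current and max health and passes them to the widget's RefreshHealthBar, after validity checks on both.
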(event EventBeginPlay
  ;[1 1 1] create the main hud widget from UMG
  (bind _returnvalue (UserInterface|CreateWidget "/Game/BattleGame/HealthBar/WBP_BattleHud.WBP_BattleHud_C" (Variables|Default|GetPlayerOwner)))
  (bind _output_get (Variables|Default|SetMainHudMenu _returnvalue))
  (UserInterface|Viewport|AddtoViewport _output_get 0)
  ;[1 1 1] save reference to player
  (bind _asbattle_game_character (Utilities|Casting|CastToBattleGameCharacter (Pawn|GetControlledPawn (Variables|Default|GetPlayerOwner))))
  (Variables|Default|SetBattlePawn _asbattle_game_character))

(event Collision|EventActorBeginOverlap
  (params (OtherActor :type Actor%20Object%20Reference)))

(event EventTick
  (params (DeltaSeconds :type Float%20%28single-precision%29))
  ;[1 1 1] refresh health bar every frame
  (bind _battlepawn (Variables|Default|GetBattlePawn)
    (:then
      (bind _mainhudmenu (Variables|Default|GetMainHudMenu)
        (:then
          (Default|RefreshHealthBar _mainhudmenu (Variables|/Script/BattleGame.BattleGameCharacter|GetHealth _battlepawn) (Variables|/Script/BattleGame.BattleGameCharacter|GetMaxHealth _battlepawn)))
        (:else)))
    (:else)))

(fn ConstructionScript)