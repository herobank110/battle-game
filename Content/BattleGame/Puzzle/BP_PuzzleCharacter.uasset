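; BP_PuzzleCharacter is a two-player race puzzle piece where dealing damage raises the attacker's marker toward a finish line.
; AnyDamage moves P1Marker or P2Marker up a step, treating player controller 0 (the listen-server host) as player one and any other instigator as player two.
; Tick checks marker heights, records the first winner, recolors the Ceiling in that player's material and disables itself.
; Once WinnerIndex is set, further damage is ignored.
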(event EventTick
  (params (DeltaSeconds :type Float%20%28single-precision%29))
  (bind _ceiling (Variables|Default|GetCeiling))
  ;[1 1 1] check if a player has won
  (if (CallFunction|HasReachedFinishLine (Variables|Default|GetP1Marker))
    (Variables|Default|SetWinnerIndex 0)
    (Rendering|Material|SetMaterial _ceiling 0 "/Game/BattleGame/Puzzle/MI_PuzzlePiece_P1.MI_PuzzlePiece_P1")
    (Actor|Tick|SetActorTickEnabled false :!label _label) ; stop checking if player has won
    (elif (CallFunction|HasReachedFinishLine (Variables|Default|GetP2Marker))
      (Variables|Default|SetWinnerIndex 1)
      (Rendering|Material|SetMaterial _ceiling 0 "/Game/BattleGame/Puzzle/MI_PuzzlePiece_P2.MI_PuzzlePiece_P2")
      (goto _label))))

(event Game|Damage|EventAnyDamage
  (params (Damage :type Float%20%28single-precision%29) (DamageType :type Damage%20Type%20Object%20Reference) (InstigatedBy :type Controller%20Object%20Reference) (DamageCauser :type Actor%20Object%20Reference))
  (bind _returnvalue (Game|GetPlayerController 0))
  (bind _p1marker (Variables|Default|GetP1Marker))
  (bind _p2marker (Variables|Default|GetP2Marker))
  (bind _returnvalue_2 (== InstigatedBy _returnvalue))
  (bind _returnvalue_3 (select _returnvalue_2 _p1marker _p2marker))
  ;[1 1 1] Move player marker up when damaged according to who instigated the damage
  (if (< (Variables|Default|GetWinnerIndex) 0) ; nobody has won yet
    (Components|MoveComponentTo _returnvalue_3 (+ (Variables|/Script/Engine.SceneComponent|GetRelativeLocation _returnvalue_3) "0, 0,20.000000") "0, 0, 0" false false 0.2 false)))

(fn ConstructionScript)

(fn HasReachedFinishLine
  (params (Marker :type Scene%20Component%20Object%20Reference))
  (return (>= (.Z (Math|Vector|BreakVector (Variables|/Script/Engine.SceneComponent|GetRelativeLocation Marker))) 105.0)))